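; Chasing enemy that pursues the player and can be killed through hits on its head collision.
; Tick checks player distance and, within a fixed radius, steers straight at the player with movement input and look-at rotation, without pathfinding.
; A hit from the player character launches that character, costs one Health and destroys the enemy at zero.
; An AI move back to the spawn location exists, but nothing here calls it.
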(event Custom|FollowPlayer
  (bind _returnvalue (Transformation|GetActorLocation))
  (bind _returnvalue_2 (Game|Player|GetPlayerPawn 0))
  (bind _returnvalue_3 (Transformation|GetActorLocation _returnvalue_2))
  ;[1 1 1] Follow Player
  (Pawn|Input|AddMovementInput (Math|Vector|Normalize (- (Math|Vector|MakeVector (.x _returnvalue_3) (.y _returnvalue_3) (.z _returnvalue_3)) (Math|Vector|MakeVector (.x _returnvalue) (.y _returnvalue) (.z _returnvalue)))) 1.0 false)
  (Transformation|SetActorRotation (Math|Rotator|FindLookatRotation (Math|Vector|MakeVector (.x _returnvalue) (.y _returnvalue) 0.0) (Math|Vector|MakeVector (.x _returnvalue_3) (.y _returnvalue_3) 0.0)))
  (Variables|Default|SetFollowingPlayer true))

(event Custom|Find%20Distance
  (bind _asbp_third_person_character (Utilities|Casting|CastToBP_ThirdPersonCharacter (Game|GetPlayerCharacter 0)))
  (bind _output_get (Variables|Default|SetDistanceFromPlayer (Transformation|GetDistanceTo _asbp_third_person_character)))
  (if (< _output_get 5e+02)
    (Variables|Default|SetSeesPawn true)
    (CallFunction|FollowPlayer)
    (else
      (Variables|Default|SetSeesPawn false))))

(event Custom|Return)

(event Custom|ReturnToStart
  (AI|Navigation|MovetoLocation (AI|GetAIController 0) (Variables|Default|GetStartLocation) -1.0 true true false true 0))

(event EventTick
  (params (DeltaSeconds :type Float%20%28single-precision%29))
  (CallFunction|FindDistance)
  (if (Variables|Default|GetSeesPawn)
    (CallFunction|FollowPlayer)
    (elif (Variables|Default|GetFollowingPlayer)
      _)))

(event Collision|EventHit
  (params (MyComp :type Primitive%20Component%20Object%20Reference) (Other :type Actor%20Object%20Reference) (OtherComp :type Primitive%20Component%20Object%20Reference) (bSelfMoved :type Boolean) (HitLocation :type Vector :default "0, 0, 0") (HitNormal :type Vector :default "0, 0, 0") (NormalImpulse :type Vector :default "0, 0, 0") (Hit :type Hit%20Result%20Structure%20%28by%20ref%29))
  ;[1 1 1] Head Collision
  (bind _asbp_third_person_character (Utilities|Casting|CastToBP_ThirdPersonCharacter Other))
  (Character|LaunchCharacter _asbp_third_person_character (Variables|Default|GetLaunchDirection) false false)
  (Variables|Default|SetHealth (- (Variables|Default|GetHealth) 1))
  (if (<= (Variables|Default|GetHealth) 0)
    (Actor|DestroyActor)))

(event EventBeginPlay
  (Variables|Default|SetStartLocation (Transformation|GetActorLocation)))

(fn ConstructionScript)