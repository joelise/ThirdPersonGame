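; Enemy character that chases the third-person player within a short radius and otherwise heads back to its spawn location.
; Tick measures player distance, then steers with raw movement input and rotation rather than AI navigation.
; The arrival stop depends on AtStart, which no live logic sets; several older return-home fragments are unused.
; Any hit with the player launches them and costs the enemy health, destroying it at zero.
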(event Custom|GoHome
  (bind _returnvalue (Transformation|GetActorLocation))
  (bind _startlocation (Variables|Default|GetStartLocation))
  (Pawn|Input|AddMovementInput (Math|Vector|Normalize (- (Math|Vector|MakeVector (.x (.location _startlocation)) (.y (.location _startlocation)) (.z (.location _startlocation))) (Math|Vector|MakeVector (.x _returnvalue) (.y _returnvalue) (.z _returnvalue)))) 1.0 false)
  (Transformation|SetActorRotation (Math|Transform|InverseTransformRotation (Transformation|GetActorTransform) (Transformation|GetActorRotation)))
  (Variables|Default|SetFollowingPlayer false))

(event Custom|Find%20Distance
  ;[1 1 1] Find Player Distance
  (bind _asbp_third_person_character (Utilities|Casting|CastToBP_ThirdPersonCharacter (Game|GetPlayerCharacter 0)))
  (bind _output_get (Variables|Default|SetDistanceFromPlayer (Transformation|GetDistanceTo _asbp_third_person_character)))
  (if (< _output_get 5e+02)
    (Variables|Default|SetSeesPawn true)
    (CallFunction|FollowPlayer)
    (else
      (Variables|Default|SetSeesPawn false))))

(event Custom|Return
  (bind _startlocation (Variables|Default|GetStartLocation))
  ;[1 1 1] Return Home
  (bind _output_get (Variables|Default|SetEnemyLocation (Transformation|GetActorLocation)))
  (Variables|Default|SetDistanceFromStart (Math|Vector|Distance(Vector) _output_get (.location (Variables|Default|GetStartLocation))))
  (Utilities|FlowControl|Sequence
    (:then_0
      (Pawn|Input|AddMovementInput (.location _startlocation) 1.0 false))
    (:then_1
      (Transformation|SetActorRotation (.rotation _startlocation))))
  (if (<= (Variables|Default|GetDistanceFromStart) 5e+02)
    _))

(event Custom|ToStart
  (if (not (Variables|Default|GetAtStart))
    (Utilities|FlowControl|Sequence
      (:then_0
        (Pawn|Input|AddMovementInput (Math|Vector|Normalize (.location (Variables|Default|GetStartLocation))) 1.0 false))
      (:then_1
        (Transformation|SetActorRotation (.rotation (Variables|Default|GetStartLocation)))))))

(event Custom|FollowPlayer
  (bind _returnvalue (Game|Player|GetPlayerPawn 0))
  (bind _returnvalue_2 (Transformation|GetActorLocation))
  (bind _returnvalue_3 (Transformation|GetActorLocation _returnvalue))
  ;[1 1 1] Follow Player
  (Pawn|Input|AddMovementInput (Math|Vector|Normalize (- (Math|Vector|MakeVector (.x _returnvalue_3) (.y _returnvalue_3) (.z _returnvalue_3)) (Math|Vector|MakeVector (.x _returnvalue_2) (.y _returnvalue_2) (.z _returnvalue_2)))) 1.0 false)
  (Transformation|SetActorRotation (Math|Rotator|FindLookatRotation (Math|Vector|MakeVector (.x _returnvalue_2) (.y _returnvalue_2) 0.0) (Math|Vector|MakeVector (.x _returnvalue_3) (.y _returnvalue_3) 0.0)))
  (Variables|Default|SetFollowingPlayer true)
  (Variables|Default|SetBegin false))

(event EventTick
  (params (DeltaSeconds :type Float%20%28single-precision%29))
  (CallFunction|FindDistance)
  (if (Variables|Default|GetSeesPawn)
    (CallFunction|FollowPlayer)
    (Variables|Default|SetBegin false)
    (else
      (if (Variables|Default|GetFollowingPlayer)
        _
        (else
          _))
      (if (Variables|Default|GetAtStart)
        (CallFunction|GoHome)
        (if (Utilities|Operators|EqualEqual (.location (Variables|Default|GetStartLocation)) (Transformation|GetActorLocation) 5.0)
          (Variables|Default|SetBegin true)
          (if (Variables|Default|GetBegin)
            (Class|NavMovementComponent|StopActiveMovement (Variables|Character|GetCharacterMovement))
            (else
              (CallFunction|GoHome))))
        (else
          (CallFunction|GoHome))))))

(event Collision|EventHit
  (params (MyComp :type Primitive%20Component%20Object%20Reference) (Other :type Actor%20Object%20Reference) (OtherComp :type Primitive%20Component%20Object%20Reference) (bSelfMoved :type Boolean) (HitLocation :type Vector :default "0, 0, 0") (HitNormal :type Vector :default "0, 0, 0") (NormalImpulse :type Vector :default "0, 0, 0") (Hit :type Hit%20Result%20Structure%20%28by%20ref%29))
  ;[1 1 1] Head Collision
  (bind _asbp_third_person_character (Utilities|Casting|CastToBP_ThirdPersonCharacter Other))
  (Character|LaunchCharacter _asbp_third_person_character (Variables|Default|GetLaunchDirection) false false)
  (Variables|Default|SetHealth (- (Variables|Default|GetHealth) 1))
  (if (<= (Variables|Default|GetHealth) 0)
    (Actor|DestroyActor)))

(event EventBeginPlay
  (bind _returnvalue (Transformation|GetActorTransform))
  ;[1 1 1] SetUp
  (Variables|Default|SetStartLocation (Math|Transform|MakeTransform (.location _returnvalue) (.rotation _returnvalue) "1.000000,1.000000,1.000000"))
  (Variables|Default|SetBegin true))

(fn ConstructionScript)