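; BP_EnemyLocation is an area actor that tracks whether the BP_ChasingEnemy is at its start location.
; On BeginPlay it finds that enemy by class and flags it as AtStart.
; The Area overlap events, filtered to that enemy, set AtStart on entry and clear it on exit, with exit also calling the enemy's Return function.
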(event OnComponentEndOverlap(Area)
  (params (OverlappedComponent :type Primitive%20Component%20Object%20Reference) (OtherActor :type Actor%20Object%20Reference) (OtherComp :type Primitive%20Component%20Object%20Reference) (OtherBodyIndex :type Integer))
  (bind _returnvalue (Actor|GetActorOfClass "/Game/_MyContent/BP_ChasingEnemy.BP_ChasingEnemy_C"))
  (if (== _returnvalue OtherActor)
    (Variables|/Game/_MyContent/BP_ChasingEnemy.BP_ChasingEnemy_C|SetAtStart _returnvalue false)
    (Default|Return _returnvalue)))

(event OnComponentBeginOverlap(Area)
  (params (OverlappedComponent :type Primitive%20Component%20Object%20Reference) (OtherActor :type Actor%20Object%20Reference) (OtherComp :type Primitive%20Component%20Object%20Reference) (OtherBodyIndex :type Integer) (bFromSweep :type Boolean) (SweepResult :type Hit%20Result%20Structure%20%28by%20ref%29))
  (bind _returnvalue (Actor|GetActorOfClass "/Game/_MyContent/BP_ChasingEnemy.BP_ChasingEnemy_C"))
  (if (== OtherActor _returnvalue)
    (Variables|/Game/_MyContent/BP_ChasingEnemy.BP_ChasingEnemy_C|SetAtStart _returnvalue true)))

(event EventBeginPlay
  (bind _returnvalue (Actor|GetActorOfClass "/Game/_MyContent/BP_ChasingEnemy.BP_ChasingEnemy_C"))
  (Variables|/Game/_MyContent/BP_ChasingEnemy.BP_ChasingEnemy_C|SetAtStart _returnvalue true))

(fn ConstructionScript)