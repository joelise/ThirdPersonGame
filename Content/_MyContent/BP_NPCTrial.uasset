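; Trial NPC Blueprint that passes proximity state and dialogue text to BP_ThirdPersonCharacter.
; SM_TriggerZone overlaps toggle PlayerNear and the character's InRange and NPCTalking flags; leaving also calls ResetDialogue.
; ResetDialogue restarts UpdateDialogue, which recurses through the Dialogue array without delay, leaving the last line as CurrentDialogueText.
; Check prints a debug greeting when the player is near; several disconnected leftovers, including a Delay, never run.
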(event OnComponentBeginOverlap(SM_TriggerZone)
  (params (OverlappedComponent :type Primitive%20Component%20Object%20Reference) (OtherActor :type Actor%20Object%20Reference) (OtherComp :type Primitive%20Component%20Object%20Reference) (OtherBodyIndex :type Integer) (bFromSweep :type Boolean) (SweepResult :type Hit%20Result%20Structure%20%28by%20ref%29))
  (bind _asbp_third_person_character (Utilities|Casting|CastToBP_ThirdPersonCharacter OtherActor))
  (Variables|/Game/ThirdPerson/Blueprints/BP_ThirdPersonCharacter.BP_ThirdPersonCharacter_C|SetInRange _asbp_third_person_character true)
  (Variables|/Game/ThirdPerson/Blueprints/BP_ThirdPersonCharacter.BP_ThirdPersonCharacter_C|SetNPCTalking _asbp_third_person_character true)
  (Variables|Default|SetPlayerNear true))

(event OnComponentEndOverlap(SM_TriggerZone)
  (params (OverlappedComponent :type Primitive%20Component%20Object%20Reference) (OtherActor :type Actor%20Object%20Reference) (OtherComp :type Primitive%20Component%20Object%20Reference) (OtherBodyIndex :type Integer))
  (bind _asbp_third_person_character (Utilities|Casting|CastToBP_ThirdPersonCharacter OtherActor))
  (Variables|/Game/ThirdPerson/Blueprints/BP_ThirdPersonCharacter.BP_ThirdPersonCharacter_C|SetInRange _asbp_third_person_character false)
  (Variables|/Game/ThirdPerson/Blueprints/BP_ThirdPersonCharacter.BP_ThirdPersonCharacter_C|SetNPCTalking _asbp_third_person_character false)
  (Variables|Default|SetPlayerNear false)
  (CallFunction|ResetDialogue))

(event Custom|UpdateDialogue
  (bind _asbp_third_person_character (Utilities|Casting|CastToBP_ThirdPersonCharacter (Game|GetPlayerCharacter 0)))
  (Variables|/Game/ThirdPerson/Blueprints/BP_ThirdPersonCharacter.BP_ThirdPersonCharacter_C|SetCurrentDialogueText _asbp_third_person_character (Utilities|Array|Get(acopy) (Variables|Default|GetDialogue) (Variables|Default|GetCurrentDialogue)))
  (Variables|Default|SetCurrentDialogue (+ (Variables|Default|GetCurrentDialogue) 1))
  (if (!= (Variables|Default|GetCurrentDialogue) (Utilities|Array|Length (Variables|Default|GetDialogue)))
    (CallFunction|UpdateDialogue)))

(event Custom|ResetDialogue
  (Variables|Default|SetCurrentDialogue 0)
  (CallFunction|UpdateDialogue))

(event Custom|Check
  (if (Variables|Default|GetPlayerNear)
    (Development|PrintString "Hello")))

(event EventBeginPlay
  (Variables|Default|SetPlayerNear false))

(event Collision|EventActorBeginOverlap
  (params (OtherActor :type Actor%20Object%20Reference)))

(event Collision|EventActorEndOverlap
  (params (OtherActor :type Actor%20Object%20Reference)))

(fn ConstructionScript)